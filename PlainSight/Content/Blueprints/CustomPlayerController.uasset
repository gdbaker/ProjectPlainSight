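; Player controller that manages the big map and scoreboard widgets for the player.
; Open_Map shows BIGMap for up to five seconds or until release, then a looping one-second timer counts down its cooldown and clears itself at zero.
; Holding Tab shows a ScoreBoard, while ScoreBoardEnd and DestroyBoardEnd events show and remove a separately referenced copy, with the former first removing the Tab board.
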(event Custom|ScoreBoardEnd
  (CallFunction|DisplayScoreBoard))

(event Custom|MapNotOnCd
  (Utilities|Time|ClearandInvalidateTimerbyHandle (stale Input|ActionEvents|InputActionOpen_Map _returnvalue)))

(event Custom|DestroyBoardEnd
  (CallFunction|DestroyScoreBoard))

(event EventBeginPlay
  (Development|PrintString "asdello"))

(event EventTick
  (params (DeltaSeconds :type Float%20%28single-precision%29)))

(event Input|ActionEvents|InputActionOpen_Map
  (params (Key :type Key%20Structure))
  (:Pressed
    (if (<= (Variables|Default|GetMapOnCd) 0)
      (Variables|Default|SetMapOnCd 20)
      (bind _returnvalue (Utilities|Time|SetTimerbyFunctionName 0 "MapCooldown" 1.0 true))
      (bind _returnvalue_2 (UserInterface|CreateWidget "/Game/UI/BIGMap.BIGMap_C"))
      (bind _output_get (Variables|Default|SetMapRef _returnvalue_2))
      (UserInterface|Viewport|AddtoViewport _output_get 0)
      (Utilities|FlowControl|Delay 5.0)
      (Widget|RemovefromParent (Variables|Default|GetMapRef))))
  (:Released
    (if (not (<= (Variables|Default|GetMapOnCd) 0))
      (Widget|RemovefromParent (Variables|Default|GetMapRef)))))

(event Input|KeyboardEvents|Tab
  (params (Key :type Key%20Structure))
  (:Pressed
    (bind _returnvalue (UserInterface|CreateWidget "/Game/UI/ScoreBoard.ScoreBoard_C"))
    (bind _output_get (Variables|Default|SetBoardRef _returnvalue))
    (UserInterface|Viewport|AddtoViewport _output_get 0))
  (:Released
    (Widget|RemovefromParent (Variables|Default|GetBoardRef))))

(fn ConstructionScript)

(fn DisplayScoreBoard
  (Widget|RemovefromParent (Variables|Default|GetBoardRef))
  (bind _returnvalue (UserInterface|CreateWidget "/Game/UI/ScoreBoard.ScoreBoard_C"))
  (bind _output_get (Variables|Default|SetScoreBoardPCRef _returnvalue))
  (UserInterface|Viewport|AddtoViewport _output_get 0))

(fn DestroyScoreBoard
  (Widget|RemovefromParent (Variables|Default|GetScoreBoardPCRef)))

(fn MapCooldown
  (Variables|Default|SetMapOnCd (- (Variables|Default|GetMapOnCd) 1))
  (if (<= (Variables|Default|GetMapOnCd) 0)
    (CallFunction|MapNotonCd)))