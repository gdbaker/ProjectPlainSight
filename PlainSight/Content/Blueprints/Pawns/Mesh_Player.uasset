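; Player character for PlainSight, handling movement, jumping, melee attack, invisibility and suicide input, plus HUD and pause menu creation.
; Movement axes route through Multiplayer-named events, and left/right input both yaws and strafes.
; Attack input sets IsAttacking on the PlayerState, and while set, Tick sends blade endpoints to player controller 0's CallAttack.
; That controller also handles invisibility and suicide, while events here play the attack montage and swap visibility materials.
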(event Custom|Attacking_replicate
  (Animation|Montage|MontagePlay (Components|SkeletalMesh|GetAnimInstance (Variables|Character|GetMesh)) "/Game/Animations/TTP_Animations/Attack_Montage.Attack_Montage" 1.0 "MontageLength" 0.3))

(event Custom|Attaking
  (Animation|Montage|MontagePlay (Components|SkeletalMesh|GetAnimInstance (Variables|Character|GetMesh)) "/Game/Animations/TTP_Animations/Attack_Montage.Attack_Montage" 1.0 "MontageLength" 0.3))

(event Custom|Multiplayer_Forward_Backward
  (params (NewParam :type Float%20%28single-precision%29))
  (Pawn|Input|AddMovementInput (Transformation|GetActorForwardVector) NewParam false))

(event Custom|Multiplayer_Left_Right
  (params (NewParam :type Float%20%28single-precision%29))
  (Pawn|Input|AddControllerYawInput NewParam)
  (Pawn|Input|AddMovementInput (Transformation|GetActorRightVector) NewParam false))

(event EventDestroyed
  (Class|SkinnedMeshComponent|SetSkeletalMesh (Variables|Character|GetMesh) "/Game/StarterContent/Blueprints/GenericMale.GenericMale" true))

(event EventOpacityvisible
  (Rendering|Material|SetMaterial (Variables|Character|GetMesh) 0 "/Game/Characters/HeroTPP/Box001_auv1_invisible.Box001_auv1_invisible"))

(event EventOpacityinvisible
  (Rendering|Material|SetMaterial (Variables|Character|GetMesh) 0 "/Game/Characters/HeroTPP/Box001_auv.Box001_auv"))

(event EventTick
  (params (DeltaSeconds :type Float%20%28single-precision%29))
  (bind _asplain_sight_player_state (Utilities|Casting|CastToPlainSightPlayerState (Variables|Default|GetPlayerState)))
  (if (Variables|/Script/PlainSight.PlainSightPlayerState|GetIsAttacking _asplain_sight_player_state)
    (bind _asplain_sight_player_controller (Utilities|Casting|CastToPlainSightPlayerController (Game|GetPlayerController 0)))
    (Class|PlainSightPlayerController|CallAttack _asplain_sight_player_controller (Transformation|GetWorldLocation (Variables|Default|GetBlade_Begin)) (Transformation|GetWorldLocation (Variables|Default|GetBlade_End)))))

(event EventBeginPlay
  (Input|EnableInput (Game|GetPlayerController 0))
  (bind _returnvalue (UserInterface|CreateWidget "/Game/UI/HUD.HUD_C"))
  (bind _output_get (Variables|Default|SetHUDReference _returnvalue))
  (UserInterface|Viewport|AddtoViewport _output_get 0))

(event Input|ActionEvents|InputActionJump
  (params (Key :type Key%20Structure))
  (:Pressed
    (Character|Jump)
    (Variables|Default|SetLanded false))
  (:Released
    (Character|StopJumping)
    (Variables|Default|SetLanded true)))

(event Input|ActionEvents|InputActionAttack
  (params (Key :type Key%20Structure))
  (:Pressed
    (bind _asplain_sight_player_state (Utilities|Casting|CastToPlainSightPlayerState (Variables|Default|GetPlayerState)))
    (Variables|/Script/PlainSight.PlainSightPlayerState|SetIsAttacking _asplain_sight_player_state true))
  (:Released
    (bind _asplain_sight_player_state_2 (Utilities|Casting|CastToPlainSightPlayerState (Variables|Default|GetPlayerState)))
    (Variables|/Script/PlainSight.PlainSightPlayerState|SetIsAttacking _asplain_sight_player_state_2 false)))

(event Input|AxisEvents|InputAxisNormal_Forward_Backward
  (params (AxisValue :type Float%20%28single-precision%29))
  (CallFunction|MultiplayerForwardBackward AxisValue))

(event Input|AxisEvents|InputAxisNormal_Left_Right
  (params (AxisValue :type Float%20%28single-precision%29))
  (CallFunction|MultiplayerLeftRight AxisValue))

(event Input|KeyboardEvents|Escape
  (params (Key :type Key%20Structure))
  (bind _returnvalue (Game|GetPlayerController 0))
  (:Pressed
    (Utilities|IsValid (Variables|Default|GetPauseMenuRef)
      (:Is%20Valid
        _)
      (:Is%20Not%20Valid
        (bind _returnvalue_2 (UserInterface|CreateWidget "/Game/UI/PauseMenu.PauseMenu_C"))
        (bind _output_get (Variables|Default|SetPauseMenuRef _returnvalue_2))))
    (Variables|/Script/Engine.PlayerController|SetbShowMouseCursor _returnvalue true)
    (Input|SetInputModeUIOnly _returnvalue _output_get "LockOnCapture")
    (UserInterface|Viewport|AddtoViewport _output_get 0)
    (Game|SetGamePaused false)))

(event Input|KeyboardEvents|P
  (params (Key :type Key%20Structure))
  (:Pressed
    (bind _asplain_sight_player_controller (Utilities|Casting|CastToPlainSightPlayerController (Game|GetPlayerController 0)))
    (Class|PlainSightPlayerController|Suicide _asplain_sight_player_controller)))

(event Input|KeyboardEvents|E
  (params (Key :type Key%20Structure))
  (:Pressed
    (bind _asplain_sight_player_controller (Utilities|Casting|CastToPlainSightPlayerController (Game|GetPlayerController 0)))
    (Class|PlainSightPlayerController|MakeInvisible _asplain_sight_player_controller)
    (Effects|SpawnEmitteratLocation "/Game/Characters/Textures/EMP_P.EMP_P" (Transformation|GetWorldLocation (Variables|Character|GetMesh)))))

(fn ConstructionScript)