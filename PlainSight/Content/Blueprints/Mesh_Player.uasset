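; Player character Blueprint that handles walking input and plays snow footstep sounds.
; Forward/back and strafe axes add movement input; DoOnce gates on forward/back input start looping timers for footsteps and floor checks, with zero-input checks clearing or restarting them.
; The Running timer function picks a left or right snow step through a random MultiGate.
; Checkfloor traces downward, but its snow-surface sound switch is disconnected, so the trace result goes unused.
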(event EventBeginPlay)

(event Collision|EventActorBeginOverlap
  (params (OtherActor :type Actor%20Object%20Reference)))

(event Input|AxisEvents|InputAxisNormal_Forward_Backward
  (params (AxisValue :type Float%20%28single-precision%29))
  (Pawn|Input|AddMovementInput (Transformation|GetActorForwardVector) AxisValue false)
  (if (or (> AxisValue 0.0) (< AxisValue 0.0))
    (Utilities|FlowControl|DoOnce false :!label _label
      (:Completed
        (Utilities|Time|SetTimerbyFunctionName 0 "Running" 0.3 true)
        (Utilities|Time|SetTimerbyFunctionName 0 "checkfloor" 0.1 true)))
    (elif (and (== AxisValue 0.0) (== (stale Input|AxisEvents|InputAxisNormal_Left_Right AxisValue) 0.0))
      (Utilities|Time|ClearTimerbyFunctionName 0 "checkfloor")
      (Utilities|Time|ClearTimerbyFunctionName 0 "Running")
      (Utilities|FlowControl|Sequence
        (:then_0
          (goto _label Reset))
        (:then_1
          (Utilities|FlowControl|DoOnce false) ; enters at Reset
        )))))

(event Input|AxisEvents|InputAxisNormal_Left_Right
  (params (AxisValue :type Float%20%28single-precision%29))
  (Pawn|Input|AddMovementInput (Transformation|GetActorRightVector) AxisValue false)
  (if (or (> AxisValue 0.0) (< AxisValue 0.0))
    (Utilities|FlowControl|DoOnce false :!label _label
      (:Completed
        (Utilities|Time|SetTimerbyFunctionName 0 "checkfloor" 0.3 true)
        (Utilities|Time|SetTimerbyFunctionName 0 "checkfloor" 0.1 true)))
    (elif (and (== (stale Input|AxisEvents|InputAxisNormal_Forward_Backward AxisValue) 0.0) (== AxisValue 0.0))
      (Utilities|Time|ClearTimerbyFunctionName 0 "checkfloor")
      (Utilities|Time|ClearTimerbyFunctionName 0 "Running")
      (Utilities|FlowControl|Sequence
        (:then_0
          (Utilities|FlowControl|DoOnce false) ; enters at Reset
        )
        (:then_1
          (goto _label Reset))))))

(fn ConstructionScript)

(fn Running
  (Utilities|FlowControl|MultiGate true false -1
    (:Out%200
      (Audio|PlaySoundatLocation "/Game/Sounds/Footsteps/Stereo/Left_snow_step.Left_snow_step" (Transformation|GetWorldLocation (Variables|Default|GetCapsuleComponent))))
    (:Out%201
      (Audio|PlaySoundatLocation "/Game/Sounds/Footsteps/Stereo/Right_snow_step.Right_snow_step" (Transformation|GetWorldLocation (Variables|Default|GetCapsuleComponent))))))

(fn Checkfloor
  (bind _capsulecomponent (Variables|Default|GetCapsuleComponent))
  (bind _returnvalue (Transformation|GetWorldLocation _capsulecomponent))
  (bind _outhit (Collision|LineTraceByChannel _returnvalue (- _returnvalue "0, 0,100.000000") "TraceTypeQuery1" false 0 "None")))