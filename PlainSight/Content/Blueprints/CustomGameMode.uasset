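; Game mode Blueprint that shows a scoreboard when the match enters the post-match phase.
; On WaitingPostMatch, it sets RemainingTime on the PlainSightGameState to 10 and creates a ScoreBoard widget for player controller 0 only.
; Any other state change removes the stored widget without a validity check, and every change prints a debug "Hello".
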(event EventBeginPlay)

(event EventOnSetMatchState
  (params (NewState :type Name :default "None"))
  (Development|PrintString "Hello")
  (if (Utilities|Name|Equal(Name) NewState "WaitingPostMatch")
    (bind _asplain_sight_game_state (Utilities|Casting|CastToPlainSightGameState (Game|GetGameState)))
    (Variables|/Script/PlainSight.PlainSightGameState|SetRemainingTime _asplain_sight_game_state 10)
    (bind _returnvalue (UserInterface|CreateWidget "/Game/UI/ScoreBoard.ScoreBoard_C" (Game|GetPlayerController 0)))
    (bind _output_get (Variables|Default|SetScoreBoardRef _returnvalue))
    (UserInterface|Viewport|AddtoViewport _output_get 0)
    (else
      (Widget|RemovefromParent (Variables|Default|GetScoreBoardRef)))))

(fn ConstructionScript)