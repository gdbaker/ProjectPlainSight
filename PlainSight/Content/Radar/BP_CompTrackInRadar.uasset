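; Actor component that registers its owner on the radar widget as a flying enemy, ground enemy, boss or pickup, based on RadarCategory.
; On BeginPlay it calls the matching add function on WBPRadarRef from BP_FlyingGameInstance after a short delay.
; A matching remove event unregisters the owner.
; As a placeholder example, an owner hit triggers removal, then destroys the owner after a brief delay.
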(event Custom|EventActorHit
  (params (SelfActor :type Actor%20Object%20Reference) (OtherActor :type Actor%20Object%20Reference) (NormalImpulse :type Vector) (Hit :type Hit%20Result%20Structure%20%28by%20ref%29))
  ;[1 0 0.02469] EXAMPLE - how to remove actor from Radar and destroy it. Delete this and make your own implementation
  (CallFunction|EventRemovefromRadar)
  (Utilities|FlowControl|Delay 0.2)
  (Actor|DestroyActor (Components|GetOwner)))

(event EventBeginPlay
  (CallFunction|EventAddtoRadar)
  ;[1 0 0.02469] EXAMPLE - how to remove actor from Radar and destroy it. Delete this and make your own implementation
  (Collision|AssignOnActorHit (Components|GetOwner) (delegate Custom|EventActorHit)))

(event Custom|EventAddToRadar
  (switch Utilities|FlowControl|Switch|SwitchonEnum_RadarCategories (Variables|Setup|GetRadarCategory)
    (:NewEnumerator0
      ;[1 1 1] Add Flying Enemy to Radar
      (Utilities|FlowControl|Delay 0.2)
      (bind _asbp_flying_game_instance (Utilities|Casting|CastToBP_FlyingGameInstance (Game|GetGameInstance)))
      (Default|FnAddFlyingEnemy (Variables|/Game/FreeRadar/BP_FlyingGameInstance.BP_FlyingGameInstance_C|GetWBPRadarRef _asbp_flying_game_instance) (Components|GetOwner)))
    (:NewEnumerator1
      ;[1 1 1] Add Ground Enemy to Radar
      (Utilities|FlowControl|Delay 0.1)
      (bind _asbp_flying_game_instance_2 (Utilities|Casting|CastToBP_FlyingGameInstance (Game|GetGameInstance)))
      (Default|FnAddGroundEnemy (Variables|/Game/FreeRadar/BP_FlyingGameInstance.BP_FlyingGameInstance_C|GetWBPRadarRef _asbp_flying_game_instance_2) (Components|GetOwner)))
    (:NewEnumerator2
      ;[1 1 1] Add Boss to Radar
      (Utilities|FlowControl|Delay 0.1)
      (bind _asbp_flying_game_instance_3 (Utilities|Casting|CastToBP_FlyingGameInstance (Game|GetGameInstance)))
      (Default|FnAddBoss (Variables|/Game/FreeRadar/BP_FlyingGameInstance.BP_FlyingGameInstance_C|GetWBPRadarRef _asbp_flying_game_instance_3) (Components|GetOwner)))
    (:NewEnumerator3
      ;[1 1 1] Add PickUp to Radar
      (Utilities|FlowControl|Delay 0.1)
      (bind _asbp_flying_game_instance_4 (Utilities|Casting|CastToBP_FlyingGameInstance (Game|GetGameInstance)))
      (Default|FnAddPickUp (Variables|/Game/FreeRadar/BP_FlyingGameInstance.BP_FlyingGameInstance_C|GetWBPRadarRef _asbp_flying_game_instance_4) (Components|GetOwner)))))

(event Custom|EventRemoveFromRadar
  (switch Utilities|FlowControl|Switch|SwitchonEnum_RadarCategories (Variables|Setup|GetRadarCategory)
    (:NewEnumerator0
      ;[1 1 1] Remove Flying Enemy from Radar
      (Utilities|FlowControl|Delay 0.1)
      (bind _asbp_flying_game_instance (Utilities|Casting|CastToBP_FlyingGameInstance (Game|GetGameInstance)))
      (Default|FnRemoveFlyingEnemy (Variables|/Game/FreeRadar/BP_FlyingGameInstance.BP_FlyingGameInstance_C|GetWBPRadarRef _asbp_flying_game_instance) (Components|GetOwner)))
    (:NewEnumerator1
      ;[1 1 1] Remove Ground Enemy from Radar
      (Utilities|FlowControl|Delay 0.1)
      (bind _asbp_flying_game_instance_2 (Utilities|Casting|CastToBP_FlyingGameInstance (Game|GetGameInstance)))
      (Default|FnRemoveGroundEnemy (Variables|/Game/FreeRadar/BP_FlyingGameInstance.BP_FlyingGameInstance_C|GetWBPRadarRef _asbp_flying_game_instance_2) (Components|GetOwner)))
    (:NewEnumerator2
      ;[1 1 1] Remove Boss from Radar
      (Utilities|FlowControl|Delay 0.1)
      (bind _asbp_flying_game_instance_3 (Utilities|Casting|CastToBP_FlyingGameInstance (Game|GetGameInstance)))
      (Default|FnRemoveBoss (Variables|/Game/FreeRadar/BP_FlyingGameInstance.BP_FlyingGameInstance_C|GetWBPRadarRef _asbp_flying_game_instance_3) (Components|GetOwner)))
    (:NewEnumerator3
      ;[1 1 1] Add PickUp to Radar
      (Utilities|FlowControl|Delay 0.1)
      (bind _asbp_flying_game_instance_4 (Utilities|Casting|CastToBP_FlyingGameInstance (Game|GetGameInstance)))
      (Default|FnRemovePickUp (Variables|/Game/FreeRadar/BP_FlyingGameInstance.BP_FlyingGameInstance_C|GetWBPRadarRef _asbp_flying_game_instance_4) (Components|GetOwner)))))